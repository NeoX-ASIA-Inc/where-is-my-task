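; BP_Board is a board actor that swings around its yaw axis when play begins and exposes a shelf as a spawn point.
; BeginPlay caches the Board component's world rotation, then a timeline adds its track value to the initial yaw, keeping pitch and roll.
; GetSpawnLocation returns the Shelf component's world transform.
; The click event on SwitcherCollision is an empty stub.
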(event OnClicked(SwitcherCollision)
  (params (TouchedComponent :type Primitive%20Component%20Object%20Reference) (ButtonPressed :type Key%20Structure)))

(event EventBeginPlay
  (Variables|Default|SetInitRoot (Transformation|GetWorldRotation (Variables|Default|Getboard)))
  (bind _newtrack_0 (Timeline|Timeline Play)
    (:Update
      (Transformation|SetWorldRotation (Variables|Default|Getboard) (Math|Rotator|MakeRotator (.roll (Variables|Default|GetInitRoot)) (.pitch (Variables|Default|GetInitRoot)) (+ _newtrack_0 (.yaw (Variables|Default|GetInitRoot)))) false false))
    (:Finished
      (Timeline|Timeline Stop))))

(fn ConstructionScript)

(fn GetSpawnLocation
  (return (Transformation|GetWorldTransform (Variables|Default|Getshelf))))